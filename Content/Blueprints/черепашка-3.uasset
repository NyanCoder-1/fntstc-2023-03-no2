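; Turtle actor variant that shuttles back and forth by overriding the MoveSelf function of its parent class.
; A state timer accumulates delta time and toggles between Forward and Backward once each phase's duration is reached, carrying over the remainder.
; Backward motion reuses the parent's movement by passing it negated delta time.
; The event graph holds only disabled default events.
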(event EventBeginPlay
  (|CallParentFunction) ; This node is disabled and will not be called.\nDrag off pins to build functionality.
)

(event Collision|EventActorBeginOverlap
  (params (OtherActor :type Actor%20Object%20Reference)))

(event EventTick
  (params (DeltaSeconds :type Float%20%28single-precision%29))
  (|CallParentFunction DeltaSeconds) ; This node is disabled and will not be called.\nDrag off pins to build functionality.
)

(fn ConstructionScript
  (|CallParentFunction))

(fn MoveSelf
  (params (DeltaTime :type Float%20%28single-precision%29))
  (CallFunction|AddTimer DeltaTime)
  (switch Utilities|FlowControl|Switch|Switchonчерепашка-3-States (Variables|Default|GetState)
    (:NewEnumerator0
      (CallFunction|Forward DeltaTime))
    (:NewEnumerator1
      (CallFunction|Backward DeltaTime))))

(fn AddTimer
  (params (DeltaTime :type Float%20%28single-precision%29))
  (Variables|Default|SetStateTimer (+ DeltaTime (Variables|Default|GetStateTimer))))

(fn Forward
  (params (DeltaTime :type Float%20%28single-precision%29))
  (if (>= (Variables|Default|GetStateTimer) (Variables|Default|GetMoveForwardTime))
    (Variables|Default|SetStateTimer (- (Variables|Default|GetStateTimer) (Variables|Default|GetMoveForwardTime)))
    (Variables|Default|SetState "NewEnumerator1")
    (|CallParentFunction (stale _result))
    (else
      (|CallParentFunction DeltaTime))))

(fn Backward
  (params (DeltaTime :type Float%20%28single-precision%29))
  (if (>= (Variables|Default|GetStateTimer) (Variables|Default|GetMoveBackwardTime))
    (Variables|Default|SetStateTimer (- (Variables|Default|GetStateTimer) (Variables|Default|GetMoveBackwardTime)))
    (Variables|Default|SetState "NewEnumerator0")
    (|CallParentFunction DeltaTime)
    (else
      (|CallParentFunction (* DeltaTime -1.0)))))