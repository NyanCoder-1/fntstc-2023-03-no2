(fn `AddTimer`
  (params (A :type "Float (double-precision)"))
  (set `self.StateTimer` (+ A (`self.StateTimer`)))
  (return))

(fn `Forward`
  (params (DeltaTime :type "Float (double-precision)"))
  (if (>= (`self.StateTimer`) (`self.MoveTime`))
    (set `self.StateTimer` (- (`self.StateTimer`) (`self.MoveTime`)))
    (set `self.State` "NewEnumerator1")
    (else
      (`parent.MoveSelf` (`local.DeltaTime`)))))

(fn `MoveSelf`
  (params (DeltaTime :type "Float (double-precision)"))
  (`self.AddTimer` DeltaTime)
  (switch `/Game/Blueprints/черепашка-2-States` (`self.State`)
    (:`NewEnumerator0`
      (`self.Forward` DeltaTime))
    (:`NewEnumerator1`
      (`self.Stay` 0.0))))

(fn `Stay`
  (params (DeltaTime :type "Float (double-precision)"))
  (if (>= (`self.StateTimer`) (`self.StayTime`))
    (bind _output_get (set `self.StateTimer` (- (`self.StateTimer`) (`self.StayTime`))))
    (set `self.State` "NewEnumerator0")
    (`parent.MoveSelf` _output_get)))

(fn `UserConstructionScript`
  (`parent.UserConstructionScript`))