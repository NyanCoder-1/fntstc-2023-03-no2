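; An interactable button actor that plays a press animation and triggers a linked spawner.
; ActionInteract restarts a timeline that lerps the button mesh between its start and end transforms.
; A first-frame flag makes the first timeline update play a water-drop sound and call Spawn on the Spawner, if valid.
; The construction script creates a dynamic material that applies the button's texture and normal map.
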(event `/Game/Blueprints/Interface-InteractiveObject.ActionInteract`
  (bind _spawner (`self.Spawner`))
  ;[1 1 1] Animate button
  (set `self.ButtonAnimationFirstFrame` true)
  (bind (_direction _buttonposition) (`Timeline|AnimateButton` :!via `PlayFromStart`)
    (:`Update`
      (`SceneComponent.K2_SetRelativeTransform` (`self.Button`) (`KismetMathLibrary.TLerp` (`self.StartPosition`) (`self.EndPosition`) _buttonposition) false false)
      ;;[1 1 1] Condition for first frame only
      (if (`self.ButtonAnimationFirstFrame`)
        (set `self.ButtonAnimationFirstFrame` false)
        ;[1 1 1] Play sound
        (`GameplayStatics.PlaySoundAtLocation` "/Game/Sounds/sound-of-a-drop-of-water-131023.sound-of-a-drop-of-water-131023" (`self.K2_GetActorLocation`) (struct) 1.0 1.0 0.0 null null null)
        (`/Engine/EditorBlueprintResources/StandardMacros.IsValid` _spawner
          (:`Is Valid`
            (`/Game/Blueprints/Spawner.Spawn` _spawner)))))))

(fn `UserConstructionScript`
  (bind _returnvalue (`PrimitiveComponent.CreateDynamicMaterialInstance` (`self.Button`) 0 "/Game/Geometry/Materials/Button.Button" "None"))
  (`MaterialInstanceDynamic.SetTextureParameterValue` _returnvalue "Normal" (`self.NormalMap`))
  (`MaterialInstanceDynamic.SetTextureParameterValue` _returnvalue "Texture" (`self.Texture`)))