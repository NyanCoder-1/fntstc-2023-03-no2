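; This actor is a homing projectile with fire sounds that travels to a Destination actor, playing an ignite sound when it spawns.
; Each Tick it checks its overlapping actors for the Destination, then plays a hit sound and destroys itself on a match.
; MoveSelf steps it toward the Destination's current location without sweep, using a lerp alpha of Speed times delta time over distance for constant-speed travel.
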(event `self.ReceiveBeginPlay`
  (`GameplayStatics.PlaySoundAtLocation` "/Game/Sounds/fire-ignite.fire-ignite" (`self.K2_GetActorLocation`) (struct) 1.0 1.0 0.0 null null null))

(event `self.ReceiveTick`
  (params (DeltaSeconds :type "Float (single-precision)"))
  (`self.DestryIfReachedTarget`)
  (`self.MoveSelf` DeltaSeconds))

(fn `DestryIfReachedTarget`
  (for _array_element (`self.GetOverlappingActors` "/Game/Blueprints/Target.Target_C")
    (if (== _array_element (`self.Destination`))
      (`GameplayStatics.PlaySoundAtLocation` "/Game/Sounds/fire-hit.fire-hit" (`self.K2_GetActorLocation`) (struct) 1.0 1.0 0.0 null null null)
      (`self.K2_DestroyActor`)
      (break)))
  (return))

(fn `MoveSelf`
  (params (DeltaTime :type "Float (double-precision)"))
  (bind _returnvalue (`self.K2_GetActorLocation`))
  (bind _destination (`self.Destination`))
  (bind _returnvalue_2 (`self.K2_GetActorLocation` _destination))
  (`/Engine/EditorBlueprintResources/StandardMacros.IsValid` _destination
    (:`Is Valid`
      (`self.K2_SetActorLocation` (`KismetMathLibrary.VLerp` _returnvalue _returnvalue_2 (/ (* (`self.Speed`) DeltaTime) (`KismetMathLibrary.Vector_Distance` _returnvalue _returnvalue_2)))))))

(fn `UserConstructionScript`)